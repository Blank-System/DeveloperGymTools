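; GymSection_A is a modular gym section: a labelled, coloured grid platform with an outline, configured entirely in the construction script.
; It creates a dynamic prototype-grid material, deriving the sub-grid and grid colours as darker multiples of the Colour variable.
; X and Y size the platform slightly inset and the outline slightly larger, both with negative Z scale, and SectionText fills the text render.
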(event EventBeginPlay)

(event Collision|EventActorBeginOverlap
  (params (OtherActor :type Actor%20Object%20Reference)))

(event EventTick
  (params (DeltaSeconds :type Float%20%28single-precision%29)))

(fn ConstructionScript
  (bind _colour (Variables|GymSection|GetColour))
  (Utilities|FlowControl|Sequence
    (:then_0
      ;[0.1111 0.2705 0.6094] Dynamic Material (Platform)
      (bind _returnvalue (Rendering|Material|CreateDynamicMaterialInstance "/Game/ModularGym/LevelPrototyping/Materials/PrototypeGrid_M.PrototypeGrid_M" "None" :!class /Script/Engine.KismetMaterialLibrary))
      (Rendering|Material|SetVectorParameterValue _returnvalue "SurfaceColor" _colour :!class /Script/Engine.MaterialInstanceDynamic)
      (Rendering|Material|SetVectorParameterValue _returnvalue "SubGridColor" (* _colour 0.677083) :!class /Script/Engine.MaterialInstanceDynamic)
      (Rendering|Material|SetVectorParameterValue _returnvalue "GridColor" (* _colour 0.28125) :!class /Script/Engine.MaterialInstanceDynamic)
      (Rendering|Material|SetMaterial (Variables|Default|GetPlatform_StaticMesh) 0 _returnvalue))
    (:then_1
      ;[0.1111 0.6094 0.6094] Scaling (Platform)
      (Transformation|SetRelativeScale3D (Variables|Default|GetOutline_StaticMesh) (Math|Vector|MakeVector (+ (Math|Conversions|ToFloat(Integer) (Variables|GymSection|GetX)) 0.1) (+ (Math|Conversions|ToFloat(Integer) (Variables|GymSection|GetY)) 0.1) -1.0))
      (Transformation|SetRelativeScale3D (Variables|Default|GetPlatform_StaticMesh) (Math|Vector|MakeVector (+ (Math|Conversions|ToFloat(Integer) (Variables|GymSection|GetX)) -0.1) (+ (Math|Conversions|ToFloat(Integer) (Variables|GymSection|GetY)) -0.1) -1.0)))
    (:then_2
      ;[0.6094 0.1111 0.2107] Text
      (Rendering|Components|TextRender|SetText (Variables|Default|GetTextRender) (Variables|GymSection|GetSectionText)))))