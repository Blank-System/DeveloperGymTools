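; Modular gym metrics prop: a ramp with a platform and text label that shows a given walk angle.
; The construction script derives vertical scale from the tangent of 90 minus Angle, so Angle is measured from vertical on a unit-scaled ramp.
; It applies that scale to both meshes and raises the label to match.
; The label shows the rounded angle, followed by Context text when provided.
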(fn ConstructionScript
  (bind _angle (Variables|Default|GetAngle))
  (bind _platform_staticmesh (Variables|Default|GetPlatform_StaticMesh))
  (bind _angle_2 (Variables|Default|GetAngle))
  (bind _context (Variables|Default|GetContext))
  (bind _returnvalue (- 9e+01 _angle_2))
  (bind _returnvalue_2 (Math|Float|Round _angle))
  (bind _returnvalue_3 (Math|Trig|Tan(Degrees) _returnvalue))
  (Utilities|FlowControl|Sequence
    (:then_0
      (Transformation|SetRelativeScale3D (Variables|Default|GetRamp_StaticMesh) (Math|Vector|MakeVector 1.0 1.0 _returnvalue_3))
      (Transformation|SetRelativeScale3D _platform_staticmesh (Math|Vector|MakeVector 0.96 1.0 _returnvalue_3))
      (Transformation|SetRelativeLocation _platform_staticmesh "-48.000000,-49.000000,1.000000" false false)
      (Transformation|SetRelativeLocation (Variables|Default|GetTextRender) (Math|Vector|MakeVector 0.0 -5e+01 (* _returnvalue_3 1e+02)) false false))
    (:then_1
      (Rendering|Components|TextRender|SetText (Variables|Default|GetTextRender) (select (Utilities|Text|TextIsEmpty _context) (Utilities|Text|ToText(Integer) _returnvalue_2) (Utilities|Text|FormatText "{X} - {Y}" _returnvalue_2 _context))))))