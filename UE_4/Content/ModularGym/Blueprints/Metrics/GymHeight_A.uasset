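; GymHeight_A is a modular gym metrics marker that measures and displays its height above the surface below it.
; Its construction script line-traces straight down on Visibility with a brief debug draw, storing the hit for visuals and label.
; Direction selects the look: Over stretches a thin support down by the hit distance, Solid Over stretches the height mesh, Under hides the support.
; The text shows the rounded distance, plus optional Context text.
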(event Custom|Under
  (Transformation|SetRelativeScale3D (Variables|Default|GetHeight_StaticMesh) "1.000000,1.000000,-0.100000")
  (Rendering|SetVisibility (Variables|Default|GetSupport_StaticMesh) false false)
  (Class|TextRenderComponent|SetVerticalAlignment (Variables|Default|GetTextRender) "EVRTA_TextTop")
  (Transformation|SetRelativeScale3D (Variables|Default|GetSupport_StaticMesh) (Math|Vector|MakeVector 0.1 0.1 0.0))
  (Transformation|SetRelativeTransform (Variables|Default|GetPlatform_StaticMesh) (Math|Transform|MakeTransform "-48.000000,-48.000000,1.000000" "0, 0, 0" "0.960000,0.960000,-0.120000") false false))

(event Custom|Over
  (Transformation|SetRelativeScale3D (Variables|Default|GetHeight_StaticMesh) "1.000000,1.000000,-0.100000")
  (Rendering|SetVisibility (Variables|Default|GetSupport_StaticMesh) true false)
  (Class|TextRenderComponent|SetVerticalAlignment (Variables|Default|GetTextRender) "EVRTA_TextTop")
  (Transformation|SetRelativeScale3D (Variables|Default|GetSupport_StaticMesh) (Math|Vector|MakeVector 0.1 0.1 (- 0.0 (/ (.Distance (Collision|BreakHitResult (Variables|Default|GetOutHit))) 1e+02))))
  (Transformation|SetRelativeTransform (Variables|Default|GetPlatform_StaticMesh) (Math|Transform|MakeTransform "-48.000000,-48.000000,1.000000" "0.000000,0.000000,0.000000" "0.960000,0.960000,-0.120000") false false))

(event Custom|Over%20%28Solid%29
  (Transformation|SetRelativeScale3D (Variables|Default|GetHeight_StaticMesh) "1.000000,1.000000,-0.100000")
  (Rendering|SetVisibility (Variables|Default|GetSupport_StaticMesh) true false)
  (Class|TextRenderComponent|SetVerticalAlignment (Variables|Default|GetTextRender) "EVRTA_TextTop")
  (Transformation|SetRelativeScale3D (Variables|Default|GetHeight_StaticMesh) (Math|Vector|MakeVector 1.0 1.0 (- 0.0 (/ (.Distance (Collision|BreakHitResult (Variables|Default|GetOutHit))) 1e+02))))
  (Transformation|SetRelativeTransform (Variables|Default|GetPlatform_StaticMesh) (Math|Transform|MakeTransform "-48.000000,-48.000000,1.000000" "0, 0, 0" "0.960000,0.960000,-0.120000") false false))

(fn ConstructionScript
  (bind _returnvalue (Transformation|GetActorLocation))
  (bind _context (Variables|Default|GetContext))
  (bind (_outhit _returnvalue_2) (Collision|LineTraceByChannel _returnvalue (+ _returnvalue (Math|Vector|MakeVector 0.0 0.0 -1e+05)) "TraceTypeQuery1" false 0 "ForDuration" true "(R=1.000000,G=0.000000,B=0.000000,A=1.000000)" "(R=0.000000,G=1.000000,B=0.000000,A=1.000000)" 0.1))
  (if _returnvalue_2
    (Variables|Default|SetOutHit _outhit)
    (Utilities|FlowControl|Sequence
      (:then_0
        ;[0.2557 0.4629 1] Handle visuals
        (switch Utilities|FlowControl|Switch|SwitchonGymOverOrUnder_E (Variables|Default|GetDirection)
          (:NewEnumerator0
            (CallFunction|Over))
          (:NewEnumerator1
            (CallFunction|Over(Solid)))
          (:NewEnumerator2
            (CallFunction|Under))))
      (:then_1
        ;[1 0.2557 0.2557] Set Text
        (Rendering|Components|TextRender|SetText (Variables|Default|GetTextRender) (select (Utilities|Text|TextIsEmpty _context) (Utilities|Text|ToText(Integer) (Math|Float|Round (.Distance (Collision|BreakHitResult (Variables|Default|GetOutHit))))) (Utilities|Text|FormatText "{X} - {Y}" (Math|Float|Round (.Distance (Collision|BreakHitResult (Variables|Default|GetOutHit)))) _context)))))))