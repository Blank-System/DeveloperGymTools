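; GymTriggerSection_A is a modular gym Blueprint that sizes and places a Trigger component to fit a section.
; The construction script derives the Trigger's location from X and Y, setting it just short of the X extent, centred along Y and raised off the floor.
; It scales the Trigger into a thin strip whose width follows Y.
; The event graph holds only disabled placeholder events, so this graph adds no overlap response.
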(event EventBeginPlay
  (|CallParentFunction) ; This node is disabled and will not be called.\nDrag off pins to build functionality.
)

(event Collision|EventActorBeginOverlap
  (params (OtherActor :type Actor%20Object%20Reference))
  (|CallParentFunction OtherActor) ; This node is disabled and will not be called.\nDrag off pins to build functionality.
)

(event EventTick
  (params (DeltaSeconds :type Float%20%28single-precision%29))
  (|CallParentFunction DeltaSeconds) ; This node is disabled and will not be called.\nDrag off pins to build functionality.
)

(fn ConstructionScript
  (bind _trigger (Variables|Default|GetTrigger))
  (|CallParentFunction)
  (Transformation|SetRelativeLocation _trigger (Math|Vector|MakeVector (- (* (Variables|Default|GetX) 1e+02) 3e+01) (* (Variables|Default|GetY) 5e+01) 4e+01) false false)
  (Transformation|SetRelativeScale3D _trigger (Math|Vector|MakeVector 0.25 (Math|Conversions|ToFloat(Integer) (Variables|Default|GetY)) 1.0)))