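; Width metric actor for a modular gym that shows a gap of a given Distance between two side meshes, with a text label.
; The construction script places the sides at plus and minus half Distance, with slightly inset highlight meshes.
; X scale follows the remainder of half Distance within a 50-unit step, negated on the right to mirror it.
; The label shows the rounded Distance, plus Context when set.
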(event EventBeginPlay)

(event Collision|EventActorBeginOverlap
  (params (OtherActor :type Actor%20Object%20Reference)))

(event EventTick
  (params (DeltaSeconds :type Float%20%28single-precision%29)))

(fn ConstructionScript
  (bind _distance (Variables|Gym|GetDistance))
  (bind _distance_2 (Variables|Gym|GetDistance))
  (bind _context (Variables|Gym|GetContext))
  (bind _returnvalue (Math|Float|Round _distance_2))
  (bind _returnvalue_2 (/ _distance 2.0))
  (bind _returnvalue_3 (Math|Float|%(Float) _returnvalue_2 5e+01))
  (bind _returnvalue_4 (- 0.0 _returnvalue_2))
  (bind _returnvalue_5 (/ _returnvalue_3 5e+01))
  (bind _returnvalue_6 (- 1.0 _returnvalue_5))
  (bind _returnvalue_7 (/ _returnvalue_6 2.0))
  (bind _returnvalue_8 (- 0.0 _returnvalue_7))
  (Transformation|SetRelativeLocation (Variables|Default|GetLeft_StaticMesh) (Math|Vector|MakeVector _returnvalue_2 -5e+01 -5e+01) false false)
  (Transformation|SetRelativeLocation (Variables|Default|GetRight_StaticMesh) (Math|Vector|MakeVector _returnvalue_4 -5e+01 -5e+01) false false)
  (Transformation|SetRelativeLocation (Variables|Default|GetLeftHighlight_StaticMesh) (Math|Vector|MakeVector (- _returnvalue_2 1.0) -48.0 -5e+01) false false)
  (Transformation|SetRelativeLocation (Variables|Default|GetRightHighlight_StaticMesh) (Math|Vector|MakeVector (+ _returnvalue_4 1.0) -48.0 -5e+01) false false)
  (Rendering|Components|TextRender|SetText (Variables|Default|GetTextRender) (select (Utilities|Text|TextIsEmpty _context) (Utilities|Text|ToText(Integer) _returnvalue) (Utilities|Text|FormatText "{X} - {Y}" _returnvalue _context)))
  (Transformation|SetRelativeScale3D (Variables|Default|GetLeft_StaticMesh) (Math|Vector|MakeVector _returnvalue_7 1.0 2.5))
  (Transformation|SetRelativeScale3D (Variables|Default|GetRight_StaticMesh) (Math|Vector|MakeVector _returnvalue_8 1.0 2.5))
  (Transformation|SetRelativeScale3D (Variables|Default|GetLeftHighlight_StaticMesh) (Math|Vector|MakeVector _returnvalue_7 0.96 2.48))
  (Transformation|SetRelativeScale3D (Variables|Default|GetRightHighlight_StaticMesh) (Math|Vector|MakeVector _returnvalue_8 0.96 2.48)))