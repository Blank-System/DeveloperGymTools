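; GymWalkAngle_A is a modular gym metrics prop that shows a ramp at a configurable Angle, with a text label.
; The construction script scales the ramp and platform meshes in Z by the tangent of 90 minus Angle, then positions the platform and raises the label to match.
; The label shows the rounded angle, followed by the Context text when one is set.
; The event graph has no active logic.
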(event EventBeginPlay)

(event Collision|EventActorBeginOverlap
  (params (OtherActor :type Actor%20Object%20Reference)))

(event EventTick
  (params (DeltaSeconds :type Float%20%28single-precision%29)))

(fn ConstructionScript
  (bind _angle (Variables|Gym|GetAngle))
  (bind _angle_2 (Variables|Gym|GetAngle))
  (bind _platform_staticmesh (Variables|Default|GetPlatform_StaticMesh))
  (bind _context (Variables|Gym|GetContext))
  (bind _returnvalue (Math|Float|Round _angle))
  (bind _returnvalue_2 (- 9e+01 _angle_2))
  (bind _returnvalue_3 (Math|Trig|Tan(Degrees) _returnvalue_2))
  (Utilities|FlowControl|Sequence
    (:then_0
      (Transformation|SetRelativeScale3D (Variables|Default|GetRamp_StaticMesh) (Math|Vector|MakeVector 1.0 1.0 _returnvalue_3))
      (Transformation|SetRelativeScale3D _platform_staticmesh (Math|Vector|MakeVector 0.96 1.0 _returnvalue_3))
      (Transformation|SetRelativeLocation _platform_staticmesh (Math|Vector|MakeVector -48.0 -49.0 1.0) false false)
      (Transformation|SetRelativeLocation (Variables|Default|GetTextRender) (Math|Vector|MakeVector 0.0 -5e+01 (* _returnvalue_3 1e+02)) false false))
    (:then_1
      (Rendering|Components|TextRender|SetText (Variables|Default|GetTextRender) (select (Utilities|Text|TextIsEmpty _context) (Utilities|Text|ToText(Integer) _returnvalue) (Utilities|Text|FormatText "{X} - {Y}" _returnvalue _context))))))