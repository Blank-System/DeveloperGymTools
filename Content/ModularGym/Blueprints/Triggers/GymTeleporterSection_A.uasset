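; GymTeleporterSection_A is a trigger actor that teleports player-controlled characters to a set destination when they overlap it.
; The destination is TeleportLocation, treated as an offset rotated by the actor's rotation and added to its location.
; After the unswept move, it stops movement on both the controller and the movement component so the character arrives without momentum.
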(event OnComponentBeginOverlap(Trigger)
  (params (OverlappedComponent :type Primitive%20Component%20Object%20Reference) (OtherActor :type Actor%20Object%20Reference) (OtherComp :type Primitive%20Component%20Object%20Reference) (OtherBodyIndex :type Integer) (bFromSweep :type Boolean) (SweepResult :type Hit%20Result%20Structure%20%28by%20ref%29))
  (bind _ascharacter (Utilities|Casting|CastToCharacter OtherActor))
  (if (Pawn|IsPlayerControlled _ascharacter)
    (Transformation|SetActorLocation _ascharacter (+ (Math|Vector|RotateVector (Variables|Default|GetTeleportLocation) (Transformation|GetActorRotation)) (Transformation|GetActorLocation)) false true)
    (AI|Navigation|StopMovement (Pawn|GetController _ascharacter))
    (Components|Movement|StopMovementImmediately (Pawn|GetMovementComponent _ascharacter))
    (Class|NavMovementComponent|StopActiveMovement (Pawn|GetMovementComponent _ascharacter))))

(fn ConstructionScript
  (|CallParentFunction))