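; Modular gym section variant that fits a trigger to the section's X and Y dimensions.
; After the parent construction script runs, it places the Trigger just inside the far X end, centered along Y and slightly raised.
; It scales the Trigger into a thin strip whose width follows Y.
; The event graph holds only disabled stubs, so this Blueprint adds no runtime logic of its own.
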(event EventBeginPlay)

(event Collision|EventActorBeginOverlap
  (params (OtherActor :type Actor%20Object%20Reference)))

(event EventTick
  (params (DeltaSeconds :type Float%20%28single-precision%29)))

(fn ConstructionScript
  (bind _trigger (Variables|Default|GetTrigger))
  (|CallParentFunction)
  ;[0.6094 0.2357 0.1111] Set Trigger Position
  (Transformation|SetRelativeLocation _trigger (Math|Vector|MakeVector (- (* (Variables|Default|GetX) 1e+02) 3e+01) (* (Variables|Default|GetY) 50) 4e+01) false false)
  (Transformation|SetRelativeScale3D _trigger (Math|Vector|MakeVector 0.25 (Math|Conversions|ToFloat(Integer) (Variables|Default|GetY)) 1.0)))